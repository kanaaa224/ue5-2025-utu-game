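; Roulette actor with three pocket triggers that pay out rewards when a BP_Ball falls in.
; Each overlap destroys the ball, spawns Kemuri Niagara effects and plays a shared sound.
; Pockets 1 and 2 drop BP_Medals through Delay-paced counter loops, and pocket 3 spawns BP_Gyouza in a for loop.
; Pocket 1 then resets Medal, while pocket 2 also writes Medal, leaving Medal2 depleted.
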(event `self.Holl＿Pocket01.OnComponentBeginOverlap`
  (params (OverlappedComponent :type "PrimitiveComponent Object Reference") (OtherActor :type "Actor Object Reference") (OtherComp :type "PrimitiveComponent Object Reference") (OtherBodyIndex :type Integer) (bFromSweep :type Boolean) (SweepResult :type "HitResult Structure (by ref)"))
  (bind _staticmesh (`self.StaticMesh`))
  ;[1 1 1] 別々のイベントを起こすために3つ作った
  ;;[1 1 1] ルーレットの穴に入ったら起こる処理の書く場所
  (bind _asbp_ball (cast `/Game/Game/GameObjects/Blueprints/BP_Ball` OtherActor))
  (`self.K2_DestroyActor` _asbp_ball) ; Ballを消す
  (`|ExecutionSequence`
    (:`then_0`
      (`NiagaraFunctionLibrary.SpawnSystemAttached` "/Game/Game/GameObjects/Efect/Kemuri.Kemuri" _staticmesh "None" (3880.0 2100.0 1540.0) (struct) "KeepWorldPosition" true)
      (`NiagaraFunctionLibrary.SpawnSystemAttached` "/Game/Game/GameObjects/Efect/Kemuri.Kemuri" _staticmesh "None" (3880.0 1400.0 1540.0) (struct) "KeepWorldPosition" true)
      (if (>= (`self.Medal`) 1) :!label _label
        (`|SpawnActorFromClass` "/Game/Game/GameObjects/Blueprints/BP_Medal.BP_Medal_C" (`KismetMathLibrary.MakeTransform` (5700.0 0.0 3965.0) (struct) (4.0 4.0 4.0)) "Undefined" "OverrideRootScale" null null)
        (`KismetSystemLibrary.Delay` 0.5)
        (bind _result (`/Engine/EditorBlueprintResources/StandardMacros.DecrementInt` (`self.Medal`))
          (:`  `
            (`KismetSystemLibrary.PrintString` (`KismetStringLibrary.Conv_IntToString` _result))
            (goto _label)))
        (else
          (set `self.Medal` 10))))
    (:`then_1`
      (`GameplayStatics.PlaySound2D` "/Game/Game/GameObjects/Sounds/SE/正解1.正解1" 1.0 1.0 0.0 null null :!label _label_2))))

(event `self.Holl＿Pocket02.OnComponentBeginOverlap`
  (params (OverlappedComponent :type "PrimitiveComponent Object Reference") (OtherActor :type "Actor Object Reference") (OtherComp :type "PrimitiveComponent Object Reference") (OtherBodyIndex :type Integer) (bFromSweep :type Boolean) (SweepResult :type "HitResult Structure (by ref)"))
  (bind _staticmesh1 (`self.StaticMesh1`))
  ;[1 1 1] 別々のイベントを起こすために3つ作った
  ;;[1 1 1] ルーレットの穴に入ったら起こる処理の書く場所
  (bind _asbp_ball (cast `/Game/Game/GameObjects/Blueprints/BP_Ball` OtherActor))
  (`self.K2_DestroyActor` _asbp_ball) ; Ballを消す
  (`|ExecutionSequence`
    (:`then_0`
      (`NiagaraFunctionLibrary.SpawnSystemAttached` "/Game/Game/GameObjects/Efect/Kemuri.Kemuri" _staticmesh1 "None" (3880.0 2100.0 1540.0) (struct) "KeepWorldPosition" true)
      (`NiagaraFunctionLibrary.SpawnSystemAttached` "/Game/Game/GameObjects/Efect/Kemuri.Kemuri" _staticmesh1 "None" (3880.0 1400.0 1540.0) (struct) "KeepWorldPosition" true)
      (if (>= (`self.Medal2`) 1) :!label _label_3
        (`|SpawnActorFromClass` "/Game/Game/GameObjects/Blueprints/BP_Medal.BP_Medal_C" (`KismetMathLibrary.MakeTransform` (5700.0 0.0 3965.0) (struct) (4.0 4.0 4.0)) "Undefined" "OverrideRootScale" null null)
        (`KismetSystemLibrary.Delay` 0.2)
        (bind _result (`/Engine/EditorBlueprintResources/StandardMacros.DecrementInt` (`self.Medal2`))
          (:`  `
            (`KismetSystemLibrary.PrintString` (`KismetStringLibrary.Conv_IntToString` _result))
            (goto _label_3)))
        (else
          (set `self.Medal` 20))))
    (:`then_1`
      (goto _label_2))))

(event `self.Holl＿Pocket03.OnComponentBeginOverlap`
  (params (OverlappedComponent :type "PrimitiveComponent Object Reference") (OtherActor :type "Actor Object Reference") (OtherComp :type "PrimitiveComponent Object Reference") (OtherBodyIndex :type Integer) (bFromSweep :type Boolean) (SweepResult :type "HitResult Structure (by ref)"))
  (bind _staticmesh2 (`self.StaticMesh2`))
  ;[1 1 1] 別々のイベントを起こすために3つ作った
  ;;[1 1 1] ルーレットの穴に入ったら起こる処理の書く場所
  (bind _asbp_ball (cast `/Game/Game/GameObjects/Blueprints/BP_Ball` OtherActor))
  (`self.K2_DestroyActor` _asbp_ball) ; Ballを消す
  (`|ExecutionSequence`
    (:`then_0`
      (`NiagaraFunctionLibrary.SpawnSystemAttached` "/Game/Game/GameObjects/Efect/Kemuri.Kemuri" _staticmesh2 "None" (3880.0 2100.0 1540.0) (struct) "KeepWorldPosition" true)
      (`NiagaraFunctionLibrary.SpawnSystemAttached` "/Game/Game/GameObjects/Efect/Kemuri.Kemuri" _staticmesh2 "None" (3880.0 1400.0 1540.0) (struct) "KeepWorldPosition" true)
      (for _ (range 4)
        (`|SpawnActorFromClass` "/Game/Game/GameObjects/Blueprints/BP_Gyouza.BP_Gyouza_C" (`KismetMathLibrary.MakeTransform` (5700.0 0.0 3965.0) (struct) (20.0 20.0 20.0)) "Undefined" "OverrideRootScale" null null)))
    (:`then_1`
      (goto _label_2))))

(fn `UserConstructionScript`)