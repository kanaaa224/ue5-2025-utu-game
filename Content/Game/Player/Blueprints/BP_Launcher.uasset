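; BP_Launcher is a player-controlled launcher actor that fires medals.
; It enables input on BeginPlay and records its starting yaw, then rotates from an axis input polled on Tick or stepped key and gamepad presses, within MaxAngle either side.
; Firing spends one Medal from BP_GameState, spawns a BP_Medal rolled 90 degrees, adds a ProjectileMovement component at runtime and plays a sound.
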(event `self.ReceiveBeginPlay`
  (`|ExecutionSequence`
    (:`then_0`
      (`self.initialize`))))

(event `self.ReceiveTick`
  (params (DeltaSeconds :type "Float (single-precision)"))
  (bind _returnvalue (`self.GetInputAxisKeyValue`))
  (`|ExecutionSequence`
    (:`then_0`
      (if (> _returnvalue 0.0)
        (`self.angle` 0.75)
        (elif (< _returnvalue 0.0)
          (`self.angle` -0.75))))))

(event `Key|Gamepad_FaceButton_Bottom`
  (params (Key :type "Key Structure"))
  (:`Pressed`
    (`|ExecutionSequence` :!label _label
      (:`then_0`
        (`self.fire`)))))

(event `Key|SpaceBar`
  (params (Key :type "Key Structure"))
  (:`Pressed`
    (goto _label)))

(event `Key|Gamepad_DPad_Left`
  (params (Key :type "Key Structure"))
  (:`Pressed`
    (`|ExecutionSequence` :!label _label_2
      (:`then_0`
        (`self.angle` -2.0)))))

(event `Key|Gamepad_LeftStick_Left`
  (params (Key :type "Key Structure"))
  (:`Pressed`
    (goto _label_2)))

(event `Key|A`
  (params (Key :type "Key Structure"))
  (:`Pressed`
    (goto _label_2)))

(event `Key|Left`
  (params (Key :type "Key Structure"))
  (:`Pressed`
    (goto _label_2)))

(event `Key|Gamepad_DPad_Right`
  (params (Key :type "Key Structure"))
  (:`Pressed`
    (`|ExecutionSequence` :!label _label_3
      (:`then_0`
        (`self.angle` 2.0)))))

(event `Key|Gamepad_LeftStick_Right`
  (params (Key :type "Key Structure"))
  (:`Pressed`
    (goto _label_3)))

(event `Key|D`
  (params (Key :type "Key Structure"))
  (:`Pressed`
    (goto _label_3)))

(event `Key|Right`
  (params (Key :type "Key Structure"))
  (:`Pressed`
    (goto _label_3)))

(event `initialize`
  (bind (_returnvalue_roll _returnvalue_pitch _returnvalue_yaw) (`KismetMathLibrary.BreakRotator` (`self.K2_GetActorRotation`)))
  (`|ExecutionSequence`
    (:`then_0`
      (`self.EnableInput` (`GameplayStatics.GetPlayerController` 0)))
    (:`then_1`
      (set `self.initial Angle` _returnvalue_yaw))))

(event `fire`
  (bind (_returnvalue_roll _returnvalue_pitch _returnvalue_yaw) (`KismetMathLibrary.BreakRotator` (`self.K2_GetActorRotation`)))
  (bind _medal (`/Game/Game/System/Blueprints/BP_GameState.Medal` (cast `/Game/Game/System/Blueprints/BP_GameState` (`GameplayStatics.GetGameState`) :!pure true)))
  (if (> _medal 0)
    (`/Engine/EditorBlueprintResources/StandardMacros.DecrementInt` _medal
      (:`  `
        (bind _returnvalue (`|SpawnActorFromClass` "/Game/Game/GameObjects/Blueprints/BP_Medal.BP_Medal_C" (`KismetMathLibrary.MakeTransform` (`self.K2_GetActorLocation`) (`KismetMathLibrary.MakeRotator` (+ _returnvalue_roll 90.0) _returnvalue_pitch _returnvalue_yaw) (`self.medal Size`)) "Undefined" "OverrideRootScale" null null))
        (`AddComponent|NODE_AddProjectileMovementComponent-1` :`self` _returnvalue)
        (`GameplayStatics.PlaySound2D` "/Game/Game/Player/Sounds/fire.fire" 1.0 1.0 0.0 null null)))))

(event `angle`
  (params (angle :type "Float (double-precision)"))
  (bind (_returnvalue_roll _returnvalue_pitch _returnvalue_yaw) (`KismetMathLibrary.BreakRotator` (`self.K2_GetActorRotation`)))
  (bind _max_angle (`self.max Angle`))
  (bind _initial_angle (`self.initial Angle`))
  (bind _returnvalue (+ _returnvalue_yaw angle))
  (if (`KismetMathLibrary.InRange_FloatFloat` _returnvalue (- _initial_angle _max_angle) (+ _initial_angle _max_angle))
    (`self.K2_SetActorRotation` (`KismetMathLibrary.MakeRotator` _returnvalue_roll _returnvalue_pitch _returnvalue))))

(fn `UserConstructionScript`)