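; BP_Hole is a moving hole stage actor that detects when a medal drops into it.
; Each tick it offsets itself along Y, flipping direction at bounds set on BeginPlay from its start position to a fixed distance beyond, so it slides back and forth.
; When a BP_Medal overlaps its capsule, it sets the HoleIn flag on BP_GameMode.
; The movement is a fixed step per frame, not scaled by delta time.
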(event `self.ReceiveTick`
  (params (DeltaSeconds :type "Float (single-precision)"))
  (bind (_returnvalue_x _returnvalue_y) (`KismetMathLibrary.BreakVector` (`self.K2_GetActorLocation`)))
  (bind (_returnvalue_x_2 _returnvalue_y_2) (`KismetMathLibrary.BreakVector` (`self.K2_GetActorLocation`)))
  (`self.K2_AddActorLocalOffset` (`self.MovingLocation`))
  (if (> _returnvalue_y (`self.End_Location_Y`))
    (set `self.MovingLocation` (0.0 -5.0 0.0))
    (elif (< _returnvalue_y_2 (`self.Start_Location_Y`))
      (set `self.MovingLocation` (0.0 5.0 0.0)))))

(event `self.ReceiveBeginPlay`
  (bind (_returnvalue_x _returnvalue_y) (`KismetMathLibrary.BreakVector` (`self.K2_GetActorLocation`)))
  (set `self.Start_Location_Y` _returnvalue_y)
  (set `self.End_Location_Y` (+ _returnvalue_y 1500.0)))

(event `self.Capsule.OnComponentBeginOverlap`
  (params (OverlappedComponent :type "PrimitiveComponent Object Reference") (OtherActor :type "Actor Object Reference") (OtherComp :type "PrimitiveComponent Object Reference") (OtherBodyIndex :type Integer) (bFromSweep :type Boolean) (SweepResult :type "HitResult Structure (by ref)"))
  (cast `/Game/Game/GameObjects/Blueprints/BP_Medal` OtherActor)
  (bind _asbp_game_mode (cast `/Game/Game/System/Blueprints/BP_GameMode` (`GameplayStatics.GetGameMode`)))
  (set `/Game/Game/System/Blueprints/BP_GameMode.HoleIn` true _asbp_game_mode))

(fn `UserConstructionScript`)