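; BP_ScoreCollision is a scoring trigger box that rewards medals and gyoza items that enter it.
; On overlap, it casts the actor to BP_Medal or BP_Gyouza and adds score and medals to BP_GameState, with gyoza worth more.
; Each hit plays a type-specific 2D sound and spawns a short-lived, colored BP_PointEffect text above the item.
; The overlapping actor itself is left untouched.
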(event `self.Box.OnComponentBeginOverlap`
  (params (OverlappedComponent :type "PrimitiveComponent Object Reference") (OtherActor :type "Actor Object Reference") (OtherComp :type "PrimitiveComponent Object Reference") (OtherBodyIndex :type Integer) (bFromSweep :type Boolean) (SweepResult :type "HitResult Structure (by ref)"))
  (`|ExecutionSequence`
    (:`then_0`
      (bind _asbp_medal (cast `/Game/Game/GameObjects/Blueprints/BP_Medal` OtherActor))
      (`self.add Score` 5)
      (`self.add Medal` 1)
      (`GameplayStatics.PlaySound2D` "/Game/Game/Stage/Sounds/SE/刀の鍔2.刀の鍔2" 1.0 1.0 0.0 null null)
      (bind (_returnvalue_x _returnvalue_y _returnvalue_z) (`KismetMathLibrary.BreakVector` (`self.K2_GetActorLocation` _asbp_medal)))
      (bind _returnvalue (`|SpawnActorFromClass` "/Game/Game/Stage/Blueprints/BP_PointEffect.BP_PointEffect_C" (`KismetMathLibrary.MakeTransform` (`KismetMathLibrary.MakeVector` _returnvalue_x _returnvalue_y (+ _returnvalue_z 400.0)) (struct :`Yaw` 180.0) (5.0 5.0 5.0)) "Undefined" "OverrideRootScale" null null))
      (bind _textrender (`/Game/Game/Stage/Blueprints/BP_PointEffect.TextRender` _returnvalue))
      (`TextRenderComponent.K2_SetText` _textrender (`self.point 1`))
      (`TextRenderComponent.SetTextRenderColor` _textrender (`self.color Yellow`))
      (`self.SetLifeSpan` _returnvalue 1.5))
    (:`then_1`
      (bind _asbp_gyouza (cast `/Game/Game/GameObjects/Blueprints/BP_Gyouza` OtherActor))
      (`self.add Score` 10)
      (`self.add Medal` 20)
      (`GameplayStatics.PlaySound2D` "/Game/Game/Stage/Sounds/SE/maou_se_system46.maou_se_system46" 1.0 1.0 0.0 null null)
      (bind (_returnvalue_x_2 _returnvalue_y_2 _returnvalue_z_2) (`KismetMathLibrary.BreakVector` (`self.K2_GetActorLocation` _asbp_gyouza)))
      (bind _returnvalue_2 (`|SpawnActorFromClass` "/Game/Game/Stage/Blueprints/BP_PointEffect.BP_PointEffect_C" (`KismetMathLibrary.MakeTransform` (`KismetMathLibrary.MakeVector` _returnvalue_x_2 _returnvalue_y_2 (+ _returnvalue_z_2 400.0)) (struct :`Yaw` 180.0) (5.0 5.0 5.0)) "Undefined" "OverrideRootScale" null null))
      (bind _textrender_2 (`/Game/Game/Stage/Blueprints/BP_PointEffect.TextRender` _returnvalue_2))
      (`TextRenderComponent.K2_SetText` _textrender_2 (`self.point 20`))
      (`TextRenderComponent.SetTextRenderColor` _textrender_2 (`self.color Green`))
      (`self.SetLifeSpan` _returnvalue_2 3.0))))

(event `add Score`
  (params (num :type Integer))
  (bind _asbp_game_state (cast `/Game/Game/System/Blueprints/BP_GameState` (`GameplayStatics.GetGameState`)))
  (set `/Game/Game/System/Blueprints/BP_GameState.Score` (+ (`/Game/Game/System/Blueprints/BP_GameState.Score` _asbp_game_state) num) _asbp_game_state))

(event `add Medal`
  (params (num :type Integer))
  (bind _asbp_game_state (cast `/Game/Game/System/Blueprints/BP_GameState` (`GameplayStatics.GetGameState`)))
  (set `/Game/Game/System/Blueprints/BP_GameState.Medal` (+ (`/Game/Game/System/Blueprints/BP_GameState.Medal` _asbp_game_state) num) _asbp_game_state))

(fn `UserConstructionScript`)