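; BP_Pusher is a stage actor that shuttles back and forth along the X axis.
; On BeginPlay it records its starting X and a turnaround point a fixed distance ahead.
; Every Tick it adds a constant local offset without sweep and flips the offset's sign whenever its world X passes either bound.
; Movement is per frame rather than scaled by delta time, so speed depends on frame rate.
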(event `self.ReceiveTick`
  (params (DeltaSeconds :type "Float (single-precision)"))
  (bind _returnvalue_x (`KismetMathLibrary.BreakVector` (`self.K2_GetActorLocation`)))
  (bind _returnvalue_x_2 (`KismetMathLibrary.BreakVector` (`self.K2_GetActorLocation`)))
  ;[1 1 1] 毎フレーム移動
  (`self.K2_AddActorLocalOffset` (`self.movinglocation`))
  ;[1 1 1] 移動の向きを逆にする
  (if (> _returnvalue_x (`self.EndLocationX`))
    (set `self.movinglocation` (-10.0 0.0 0.0))
    (else
      ;[1 1 1] スタート地点を越したら逆にする
      (if (< _returnvalue_x_2 (`self.Start_LocationX`))
        (set `self.movinglocation` (10.0 0.0 0.0))))))

(event `self.ReceiveBeginPlay`
  (bind _returnvalue_x (`KismetMathLibrary.BreakVector` (`self.K2_GetActorLocation`)))
  ;[1 1 1] スタート地点と折り返し地点をセット
  (set `self.EndLocationX` (+ _returnvalue_x 1180.0))
  (set `self.Start_LocationX` _returnvalue_x))

(fn `UserConstructionScript`)