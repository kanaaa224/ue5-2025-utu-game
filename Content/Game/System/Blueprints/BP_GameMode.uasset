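; BP_GameMode is the game mode that runs a two-minute countdown for the match.
; BeginPlay records the start time and limit, then Tick recomputes the whole seconds remaining from the wall clock.
; When time runs out, it sets IsEnded only if the GameMode value on BP_GameInstance is 0.
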(event `self.ReceiveBeginPlay`
  (set `self.Started Time` (`KismetMathLibrary.Now`))
  (set `self.Time Limit` (`KismetMathLibrary.MakeTimespan` 0 0 2)))

(event `self.ReceiveTick`
  (params (DeltaSeconds :type "Float (single-precision)"))
  (`|ExecutionSequence`
    (:`then_0`
      (set `self.Time Left Seconds` (`KismetMathLibrary.FTrunc` (`KismetMathLibrary.GetTotalSeconds` (- (`self.Time Limit`) (- (`KismetMathLibrary.Now`) (`self.Started Time`)))))))
    (:`then_1`
      (if (<= (`self.Time Left Seconds`) 0)
        (bind _asbp_game_instance (cast `/Game/Game/System/Blueprints/BP_GameInstance` (`GameplayStatics.GetGameInstance`)))
        (if (== (`/Game/Game/System/Blueprints/BP_GameInstance.Game Mode` _asbp_game_instance) 0)
          (set `self.Is Ended` true))))))

(fn `UserConstructionScript`)